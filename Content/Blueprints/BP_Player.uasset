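; Player ship pawn that moves within clamped bounds, banks when strafing, and manages health and a shield.
; Held fire runs a Gate and Delay loop through four cyclable weapons: single shot, triple spread, random five-shot scatter and persistent beam.
; Tick drives movement, roll, beam position and shield drain or refill, with a cooldown after depletion.
; Getters expose health and shield values and ratios; debug keys randomly alter health, and UI creation is disconnected.
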(event `InputAction|Fire`
  (params (Key :type "Key Structure"))
  (bind _returnvalue (`KismetMathLibrary.MakeRotator` 0.0 0.0 (`KismetMathLibrary.RandomFloatInRange` -25.0 25.0)))
  ;[1 1 1] Player Fire
  (:`Pressed`
    (bind _output_get (set `self.Is Firing` true))
    (if _output_get
      (`|ExecutionSequence`
        (:`then_0`
          (goto _label_2 :!via `Open`))
        (:`then_1`
          (`KismetSystemLibrary.Delay` (`KismetMathLibrary.FClamp` (* (`self.Fire_Rate`) (`self.Fire_Rate_Multi`)) 0.033) :!label _label)
          (`/Engine/EditorBlueprintResources/StandardMacros.Gate` true :!label _label_2
            (:`Exit`
              (`|ExecutionSequence`
                (:`then_0`
                  _)
                (:`then_1`
                  (goto _label)))))))
      (else
        (`|ExecutionSequence`
          (:`then_0`
            (goto _label_2 :!via `Open`))
          (:`then_1`
            (goto _label_2)))))
    (if (`self.Is Firing`)
      (if (== (`self.CurrentWeapon`) 1.0)
        (set `self.Fire_Rate` 0.1)
        (`|SpawnActorFromClass` (`self.Projectile`) (`KismetMathLibrary.MakeTransform` (`SceneComponent.GetSocketLocation` (`self.StaticMesh`) "FiringSocket")) "Undefined" "OverrideRootScale" null 1.0 3000.0 null)
        (`GameplayStatics.PlaySound2D` "/Game/Sounds/sfx_PlayerBullet_Cue.sfx_PlayerBullet_Cue" 1.0 1.0 0.0 null null)
        (elif (== (`self.CurrentWeapon`) 2.0)
          (set `self.Fire_Rate` 0.2)
          (`|SpawnActorFromClass` (`self.Projectile`) (`KismetMathLibrary.MakeTransform` (`SceneComponent.GetSocketLocation` (`self.StaticMesh`) "FiringSocket")) "Undefined" "OverrideRootScale" null 1.0 3000.0 null)
          (`|SpawnActorFromClass` (`self.Projectile`) (`KismetMathLibrary.MakeTransform` (`SceneComponent.GetSocketLocation` (`self.StaticMesh`) "FiringSocket") (struct :`Yaw` 25.0)) "Undefined" "OverrideRootScale" null 1.0 3000.0 null)
          (`|SpawnActorFromClass` (`self.Projectile`) (`KismetMathLibrary.MakeTransform` (`SceneComponent.GetSocketLocation` (`self.StaticMesh`) "FiringSocket") (struct :`Yaw` -25.0)) "Undefined" "OverrideRootScale" null 1.0 3000.0 null)
          (`GameplayStatics.PlaySound2D` "/Game/Sounds/sfx_PlayerBullet_Cue.sfx_PlayerBullet_Cue" 1.0 1.0 0.0 null null)
          (elif (== (`self.CurrentWeapon`) 3.0)
            (set `self.Fire_Rate` 0.3)
            (`|SpawnActorFromClass` (`self.Projectile`) (`KismetMathLibrary.MakeTransform` (`SceneComponent.GetSocketLocation` (`self.StaticMesh`) "FiringSocket") _returnvalue) "Undefined" "OverrideRootScale" null 1.0 3000.0 null)
            (`|SpawnActorFromClass` (`self.Projectile`) (`KismetMathLibrary.MakeTransform` (`SceneComponent.GetSocketLocation` (`self.StaticMesh`) "FiringSocket") _returnvalue) "Undefined" "OverrideRootScale" null 1.0 3000.0 null)
            (`|SpawnActorFromClass` (`self.Projectile`) (`KismetMathLibrary.MakeTransform` (`SceneComponent.GetSocketLocation` (`self.StaticMesh`) "FiringSocket") _returnvalue) "Undefined" "OverrideRootScale" null 1.0 3000.0 null)
            (`|SpawnActorFromClass` (`self.Projectile`) (`KismetMathLibrary.MakeTransform` (`SceneComponent.GetSocketLocation` (`self.StaticMesh`) "FiringSocket") _returnvalue) "Undefined" "OverrideRootScale" null 1.0 3000.0 null)
            (`|SpawnActorFromClass` (`self.Projectile`) (`KismetMathLibrary.MakeTransform` (`SceneComponent.GetSocketLocation` (`self.StaticMesh`) "FiringSocket") _returnvalue) "Undefined" "OverrideRootScale" null 1.0 3000.0 null)
            (`GameplayStatics.PlaySound2D` "/Game/Sounds/sfx_PlayerBullet_Cue.sfx_PlayerBullet_Cue" 1.0 1.0 0.0 null null)
            (elif (== (`self.CurrentWeapon`) 4.0)
              (if (not (`self.BeamOn`))
                (bind _returnvalue_2 (`|SpawnActorFromClass` (`self.Beam`) (`KismetMathLibrary.MakeTransform` (`SceneComponent.GetSocketLocation` (`self.StaticMesh`) "FiringSocket")) "Undefined" "OverrideRootScale" null 50.0 1.0 null))
                (set `self.BeamOn` true)
                (set `self.Lazer Reference` _returnvalue_2))))))))
  (:`Released`
    (set `self.Is Firing` false)
    (if (`self.BeamOn`)
      (`self.K2_DestroyActor` (`self.Lazer Reference`))
      (set `self.BeamOn` false))))

(event `InputAction|SwappingWeapons`
  (params (Key :type "Key Structure"))
  (bind _currentweapon (`self.CurrentWeapon`))
  (bind _lazer_reference (`self.Lazer Reference`))
  ;[1 1 1] Weapon Swap
  (:`Pressed`
    (`/Engine/EditorBlueprintResources/StandardMacros.DoOnce` false :!label _label_3
      (:`Completed`
        (`KismetSystemLibrary.PrintString` (`KismetStringLibrary.Conv_DoubleToString` _currentweapon))
        (if (== _currentweapon 1.0)
          (set `self.CurrentWeapon` 2.0)
          (elif (== (`self.CurrentWeapon`) 2.0)
            (set `self.CurrentWeapon` 3.0)
            (elif (== (`self.CurrentWeapon`) 3.0)
              (set `self.CurrentWeapon` 4.0)
              (elif (== (`self.CurrentWeapon`) 4.0)
                (set `self.BeamOn` false)
                (`/Engine/EditorBlueprintResources/StandardMacros.IsValid` _lazer_reference
                  (:`Is Valid`
                    (`self.K2_DestroyActor` _lazer_reference)
                    (set `self.CurrentWeapon` 1.0))))))))))
  (:`Released`
    (goto _label_3 :!via `Reset`)))

(event `InputAxis|MoveForward`
  (params (AxisValue :type "Float (single-precision)"))
  ;[1 1 1] Input
  (set `self.X Movement` AxisValue))

(event `InputAxis|MoveRight`
  (params (AxisValue :type "Float (single-precision)"))
  ;[1 1 1] Input
  (set `self.Y Movement` AxisValue))

(event `self.ReceiveTick`
  (params (DeltaSeconds :type "Float (single-precision)"))
  (bind _lazer_reference (`self.Lazer Reference`))
  ;[1 1 1] Shield Input Processing
  (if (> (`self.CurrentShield`) 0.0)
    (if (<= (`self.CurrentShieldCooldown`) 0.0)
      (if (`self.ShieldActive`)
        (`self.EditShield` (* (* (`self.ShieldUseSpeed`) -1.0) (`GameplayStatics.GetWorldDeltaSeconds`)))
        (`PrimitiveComponent.SetVisibleInSceneCaptureOnly` (`self.Shield Particle`) false)
        (else
          (`self.EditShield` (* (`self.ShieldRefillSpeed`) (`GameplayStatics.GetWorldDeltaSeconds`)))
          (`PrimitiveComponent.SetVisibleInSceneCaptureOnly` (`self.Shield Particle`) true)))
      (else
        (set `self.CurrentShieldCooldown` (- (`self.CurrentShieldCooldown`) (* (`GameplayStatics.GetWorldDeltaSeconds`) 100.0)))))
    (else
      (set `self.CurrentShieldCooldown` (`self.MaxShieldCooldown`))
      (set `self.CurrentShield` 1.0)
      (`PrimitiveComponent.SetVisibleInSceneCaptureOnly` (`self.Shield Particle`) true)))
  ;[1 1 1] Event Tick
  (`self.Move Actor` DeltaSeconds)
  (`self.Roll Ship` DeltaSeconds)
  (if (`self.BeamOn`)
    (`/Engine/EditorBlueprintResources/StandardMacros.IsValid` _lazer_reference
      (:`Is Valid`
        (`self.K2_SetActorLocation` _lazer_reference (`SceneComponent.GetSocketLocation` (`self.StaticMesh`) "FiringSocket") false true)))))

(event `self.ReceiveBeginPlay`
  ;[1 1 1] Init Variables
  (set `self.CurrentShield` (`self.MaxShield`))
  (set `self.CurrentHealth` (`self.MaxHealth`))
  (`PrimitiveComponent.SetVisibleInSceneCaptureOnly` (`self.Shield Particle`) false))

(event `Key|Comma`
  (params (Key :type "Key Structure"))
  ;[1 1 1] Health Debug
  (:`Pressed`
    (`self.EditHealth` (`KismetMathLibrary.RandomFloatInRange` -25.0 -500.0))))

(event `Key|RightMouseButton`
  (params (Key :type "Key Structure"))
  ;[1 1 1] Shield Input
  (:`Pressed`
    (set `self.ShieldActive` true))
  (:`Released`
    (set `self.ShieldActive` false)))

(event `Key|Period`
  (params (Key :type "Key Structure"))
  ;[1 1 1] Health Debug
  (:`Pressed`
    (`self.EditHealth` (`KismetMathLibrary.RandomFloatInRange` 25.0 500.0))))

(event `EditHealth`
  (params (HealthToAdd :type "Float (double-precision)"))
  ;[1 1 1] HealthFunction
  (set `self.CurrentHealth` (`KismetMathLibrary.FClamp` (+ HealthToAdd (`self.CurrentHealth`)) 0.0 (`self.MaxHealth`)))
  (`GameplayStatics.PlaySound2D` "/Game/Sounds/sfx_bigimpact.sfx_bigimpact" 1.0 1.0 0.0 null null))

(event `EditShield`
  (params (ShieldToAdd :type "Float (double-precision)"))
  ;[1 1 1] ShieldFunction
  (set `self.CurrentShield` (`KismetMathLibrary.FClamp` (+ ShieldToAdd (`self.CurrentShield`)) 0.0 (`self.MaxShield`))))

(event `SetShield`
  (params (ShieldToSet :type "Float (double-precision)"))
  ;[1 1 1] ShieldFunction
  (set `self.CurrentShield` (`KismetMathLibrary.FClamp` ShieldToSet 0.0 (`self.MaxShield`))))

(fn `GetHealth`
  (returns (Result :type "Float (double-precision)"))
  (return (`self.CurrentHealth`)))

(fn `GetHealthAsRatio`
  (returns (Result :type "Float (double-precision)"))
  (bind _result (`self.GetHealth`))
  (return (/ _result (`self.MaxHealth`))))

(fn `GetShield`
  (returns (Result :type "Float (double-precision)"))
  (return (`self.CurrentShield`)))

(fn `GetShieldAsRatio`
  (returns (Result :type "Float (double-precision)"))
  (bind _result (`self.GetShield`))
  (return (/ _result (`self.MaxShield`))))

(fn `Move Actor`
  (params (Delta :type "Float (double-precision)"))
  (bind _output_get (set `self.Move Vector` (`KismetMathLibrary.MakeVector` (`self.X Movement`) (`self.Y Movement`))))
  (`KismetMathLibrary.Vector_Normalize` _output_get 1.0)
  (`SceneComponent.K2_SetWorldLocation` (`self.DefaultSceneRoot`) (`KismetMathLibrary.MakeVector` (`KismetMathLibrary.FClamp` (.x (+ (* (`self.Move Vector`) (* Delta (`self.Speed`))) (`SceneComponent.K2_GetComponentLocation` (`self.DefaultSceneRoot`)))) (.x (`self.Min Location`)) (.x (`self.Max Location`))) (`KismetMathLibrary.FClamp` (.y (+ (* (`self.Move Vector`) (* Delta (`self.Speed`))) (`SceneComponent.K2_GetComponentLocation` (`self.DefaultSceneRoot`)))) (.y (`self.Min Location`)) (.y (`self.Max Location`))) (`KismetMathLibrary.FClamp` (.z (+ (* (`self.Move Vector`) (* Delta (`self.Speed`))) (`SceneComponent.K2_GetComponentLocation` (`self.DefaultSceneRoot`)))) (.z (`self.Min Location`)) (.z (`self.Max Location`)))) false true))

(fn `Roll Ship`
  (params (Delta :type "Float (double-precision)"))
  (bind _y_movement (`self.Y Movement`))
  (bind _staticmesh (`self.StaticMesh`))
  (if (< _y_movement 0.0)
    (bind _output_get (set `self.Current Roll` (`KismetMathLibrary.FMin` (+ (`self.Current Roll`) (* (`self.Roll Speed`) Delta)) (`self.MaxRoll`))))
    (`SceneComponent.K2_SetWorldRotation` _staticmesh (`KismetMathLibrary.MakeRotator` _output_get 0.0 0.0) false false)
    (elif (> _y_movement 0.0)
      (bind _output_get_2 (set `self.Current Roll` (`KismetMathLibrary.FMax` (- (`self.Current Roll`) (* (`self.Roll Speed`) Delta)) (* (`self.MaxRoll`) -1.0))))
      (`SceneComponent.K2_SetWorldRotation` _staticmesh (`KismetMathLibrary.MakeRotator` _output_get_2 0.0 0.0) false false)
      (else
        (bind _output_get_3 (set `self.Current Roll` (- (`self.Current Roll`) (* (* (`self.Roll Speed`) Delta) (`KismetMathLibrary.SignOfFloat` (`self.Current Roll`))))))
        (`SceneComponent.K2_SetWorldRotation` _staticmesh (`KismetMathLibrary.MakeRotator` _output_get_3 0.0 0.0) false false)))))

(fn `UserConstructionScript`)