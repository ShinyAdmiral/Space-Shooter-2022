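; Enemy projectile actor that flies at a configurable ProjectileSpeed, applied to its movement component's initial and max speed in the construction script.
; On BeginPlay it turns to face its velocity and spawns a muzzle flash effect at the mesh location.
; Overlap handling is unfinished: it switches on the other actor's first tag with no resulting actions, the boss cast is unconnected, and Destroyed is empty.
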(event `self.ReceiveBeginPlay`
  (bind _returnvalue (`self.K2_GetActorLocation`))
  (`self.K2_SetActorRotation` (`KismetMathLibrary.FindLookAtRotation` _returnvalue (+ _returnvalue (`self.GetVelocity`))))
  (`NiagaraFunctionLibrary.SpawnSystemAtLocation` "/Game/Particles/NS_MuzzleFlash.NS_MuzzleFlash" (`SceneComponent.K2_GetComponentLocation` (`self.ProjectileMesh`))))

(event `self.ReceiveActorBeginOverlap`
  (params (OtherActor :type "Actor Object Reference"))
  (switch `name` (`|GetArrayItem` (`Actor.Tags` OtherActor))))

(event `self.ReceiveDestroyed`)

(fn `UserConstructionScript`
  (bind _projectilemovement (`self.ProjectileMovement`))
  (bind _projectile_speed (`self.Projectile_Speed`))
  (set `ProjectileMovementComponent.InitialSpeed` _projectile_speed _projectilemovement)
  (set `ProjectileMovementComponent.MaxSpeed` _projectile_speed _projectilemovement))