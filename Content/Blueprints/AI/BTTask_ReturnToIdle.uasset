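; Behavior tree task that returns the boss to its starting position and idle state.
; On execute it resets the BossAttackState blackboard enum, triggers the matching controller phase and clears the boss's child actor class.
; Each tick it lerps the pawn toward the StartingLocation key without setting rotation.
; It finishes once location and summed rotation difference from the controller's InitialRotation are within tolerance.
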(event `self.ReceiveExecuteAI`
  (params (OwnerController :type "AIController Object Reference") (ControlledPawn :type "Pawn Object Reference"))
  (`BlackboardComponent.SetValueAsEnum` (`AIBlueprintHelperLibrary.GetBlackboard` OwnerController) "BossAttackState" (enumliteral `/Game/Blueprints/AI/E_BossAttacks` "NewEnumerator0"))
  (bind _asbp_boss_controller (cast `/Game/Blueprints/AI/BP_BossController` OwnerController))
  (`/Game/Blueprints/AI/BP_BossController.TriggerBossPhase` _asbp_boss_controller "NewEnumerator0")
  (bind _asbp_boss_actor (cast `/Game/Blueprints/AI/BP_BossActor` ControlledPawn))
  (`ChildActorComponent.SetChildActorClass` (`/Game/Blueprints/AI/BP_BossActor.ChildActor` _asbp_boss_actor) null))

(event `self.ReceiveTickAI`
  (params (OwnerController :type "AIController Object Reference") (ControlledPawn :type "Pawn Object Reference") (DeltaSeconds :type "Float (single-precision)"))
  (bind _returnvalue (`Actor.K2_GetActorLocation` ControlledPawn))
  (bind _returnvalue_2 (`BlackboardComponent.GetValueAsVector` (`AIBlueprintHelperLibrary.GetBlackboard` OwnerController) "StartingLocation"))
  (bind _asbp_boss_controller (cast `/Game/Blueprints/AI/BP_BossController` OwnerController))
  (`Actor.K2_SetActorLocation` ControlledPawn (`KismetMathLibrary.VLerp` _returnvalue _returnvalue_2 (* 2 DeltaSeconds)) false false)
  (bind (_returnvalue_roll _returnvalue_pitch _returnvalue_yaw) (`KismetMathLibrary.BreakRotator` (`KismetMathLibrary.NormalizedDeltaRotator` (`Actor.K2_GetActorRotation` ControlledPawn) (`/Game/Blueprints/AI/BP_BossController.InitialRotation` _asbp_boss_controller))))
  (if (and (== _returnvalue _returnvalue_2 :`ErrorTolerance` 5.0) (< (`KismetMathLibrary.Abs` (+ _returnvalue_roll _returnvalue_pitch _returnvalue_yaw)) 3.0))
    (`self.FinishExecute` true)))