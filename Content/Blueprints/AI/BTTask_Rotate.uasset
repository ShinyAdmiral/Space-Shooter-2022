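; Behavior tree task that rotates the boss pawn through its palm laser sweep over a set rotation time.
; On execute it resets a timer, then each tick accumulates delta time and lerps the pawn along the shortest path between the start and end laser rotations stored on BP_BossController.
; It finishes successfully once the timer reaches the rotation time.
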(event `self.ReceiveTickAI`
  (params (OwnerController :type "AIController Object Reference") (ControlledPawn :type "Pawn Object Reference") (DeltaSeconds :type "Float (single-precision)"))
  (set `self.Timer` (+ DeltaSeconds (`self.Timer`)))
  (bind _asbp_boss_controller (cast `/Game/Blueprints/AI/BP_BossController` OwnerController))
  (`Actor.K2_SetActorRotation` ControlledPawn (`KismetMathLibrary.RLerp` (`/Game/Blueprints/AI/BP_BossController.PalmLaserRotation` _asbp_boss_controller) (`/Game/Blueprints/AI/BP_BossController.EndPalmLaserRotation` _asbp_boss_controller) (/ (`self.Timer`) (`self.RotationTime`)) true) false)
  (if (>= (`self.Timer`) (`self.RotationTime`))
    (`self.FinishExecute` true)))

(event `self.ReceiveExecuteAI`
  (params (OwnerController :type "AIController Object Reference") (ControlledPawn :type "Pawn Object Reference"))
  (set `self.Timer` 0.0))