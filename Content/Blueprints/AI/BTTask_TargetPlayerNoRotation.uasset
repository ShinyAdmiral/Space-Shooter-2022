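; Behavior tree task that slides the boss pawn sideways to line up with the player, without changing its rotation.
; Each AI tick casts the owner to BP_BossController and builds a target from the blackboard StartingLocation's X and Z plus player 0's Y.
; The pawn eases toward that point with a delta-time-scaled lerp and no sweep.
; The task never calls Finish Execute.
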(event `self.ReceiveTickAI`
  (params (OwnerController :type "AIController Object Reference") (ControlledPawn :type "Pawn Object Reference") (DeltaSeconds :type "Float (single-precision)"))
  (bind _asbp_boss_controller (cast `/Game/Blueprints/AI/BP_BossController` OwnerController))
  (`Actor.K2_SetActorLocation` ControlledPawn (`KismetMathLibrary.VLerp` (`Actor.K2_GetActorLocation` ControlledPawn) (`KismetMathLibrary.MakeVector` (.x (`BlackboardComponent.GetValueAsVector` (`AIBlueprintHelperLibrary.GetBlackboard` _asbp_boss_controller) "StartingLocation")) (.y (`Actor.K2_GetActorLocation` (`GameplayStatics.GetPlayerPawn` 0))) (.z (`BlackboardComponent.GetValueAsVector` (`AIBlueprintHelperLibrary.GetBlackboard` _asbp_boss_controller) "StartingLocation"))) (* 4 DeltaSeconds)) false false))