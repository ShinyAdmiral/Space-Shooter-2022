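; Behavior tree task that picks the boss's next attack at random for BP_BossController.
; It rolls a random E_BossAttacks value, skipping the first entry, and rerolls while it matches the PreviousBossAttack blackboard key.
; The new value is written to both PreviousBossAttack and BossAttackState, then the task finishes successfully.
; A disconnected debug branch forces a fixed attack state for testing.
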(event `self.ReceiveExecute`
  (params (OwnerActor :type "Actor Object Reference"))
  (bind _asbp_boss_controller (cast `/Game/Blueprints/AI/BP_BossController` OwnerActor))
  (bind _output_get (set `self.RandomNewState` (cast `/Game/Blueprints/AI/E_BossAttacks` (`KismetMathLibrary.Conv_IntToByte` (`KismetMathLibrary.RandomIntegerInRange` 1 (- (enumcount `/Game/Blueprints/AI/E_BossAttacks`) 1)))) :!label _label))
  (bind _returnvalue (`AIBlueprintHelperLibrary.GetBlackboard` _asbp_boss_controller))
  (if (`|EnumEquality` _output_get (cast `/Game/Blueprints/AI/E_BossAttacks` (`BlackboardComponent.GetValueAsEnum` _returnvalue "PreviousBossAttack")))
    (goto _label)
    (else
      (`BlackboardComponent.SetValueAsEnum` _returnvalue "PreviousBossAttack" (`self.RandomNewState`))
      (`BlackboardComponent.SetValueAsEnum` _returnvalue "BossAttackState" (`self.RandomNewState`))
      (`self.FinishExecute` true))))