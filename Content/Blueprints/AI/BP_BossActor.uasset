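; BP_BossActor is a boss that takes damage from overlapping player projectiles and destroys itself when its health runs out.
; Overlaps branch on the other actor's first tag, then subtract the projectile's damage times its multiplier, run HealthCheck and destroy the projectile.
; It pushes max health to BP_Player on BeginPlay and current health every Tick.
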(event `self.ReceiveBeginPlay`
  (set `self.Health` (`self.MaxHealth`))
  (bind _asbp_player (cast `/Game/Blueprints/BP_Player` (`GameplayStatics.GetPlayerPawn` 0)))
  (set `/Game/Blueprints/BP_Player.BossMaxHealth` (`self.MaxHealth`) _asbp_player))

(event `self.ReceiveActorBeginOverlap`
  (params (OtherActor :type "Actor Object Reference"))
  (bind _asbp_player_projectile (cast `/Game/Blueprints/BP_PlayerProjectile` OtherActor :!pure true))
  (switch `name` (`|GetArrayItem` (`Actor.Tags` OtherActor))
    (:`PlayerBullet`
      (if (> (`self.Health`) 0.0)
        (set `self.Health` (- (`self.Health`) (* (`/Game/Blueprints/BP_PlayerProjectile.Damage` _asbp_player_projectile) (`/Game/Blueprints/BP_PlayerProjectile.Damage_Multi` _asbp_player_projectile))))
        (`self.Health Check`)
        (`self.K2_DestroyActor` _asbp_player_projectile)))))

(event `self.ReceiveTick`
  (params (DeltaSeconds :type "Float (single-precision)"))
  (bind _asbp_player (cast `/Game/Blueprints/BP_Player` (`GameplayStatics.GetPlayerPawn` 0)))
  (set `/Game/Blueprints/BP_Player.BossCurrentHealth` (`self.Health`) _asbp_player))

(fn `Health Check`
  (if (<= (`self.Health`) 0.0)
    (`self.K2_DestroyActor`)))

(fn `UserConstructionScript`)