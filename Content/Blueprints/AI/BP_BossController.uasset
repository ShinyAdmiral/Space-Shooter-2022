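; AI controller for a giant-hand boss with Fist, Splayed and Finger Gun attack phases.
; BeginPlay runs BT_Boss, seeds its blackboard with start location and fist speed, and caches the right hand's anim blueprint.
; TriggerBossPhase uses a timeline to blend pose weights and lerp pawn rotation toward each phase.
; SplayedMovement sweeps the pawn along Y, while ShootFunction fires a three-bullet spread or a yaw-aimed shot at the player.
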(event `self.ReceiveBeginPlay`
  (bind _returnvalue (`self.K2_GetPawn`))
  (bind _returnvalue_2 (`AIBlueprintHelperLibrary.GetBlackboard` self))
  (set `self.InitialRotation` (`self.K2_GetActorRotation` _returnvalue))
  (`self.RunBehaviorTree` "/Game/Blueprints/AI/BT_Boss.BT_Boss")
  (`BlackboardComponent.SetValueAsVector` _returnvalue_2 "StartingLocation" (`self.K2_GetActorLocation` _returnvalue))
  (`BlackboardComponent.SetValueAsFloat` _returnvalue_2 "FistSpeed" (`self.FistSpeed`))
  (bind _asbp_boss_actor (cast `/Game/Blueprints/AI/BP_BossActor` _returnvalue))
  (bind _asboss_mannequin_hand_right_skeleton_anim_blueprint (cast `/Game/Geometry/Mannequin/Character/Mesh/Boss_MannequinHand_Right_Skeleton_AnimBlueprint` (`SkeletalMeshComponent.GetAnimInstance` (`/Game/Blueprints/AI/BP_BossActor.MannequinHand_Right` _asbp_boss_actor))))
  (set `self.BossAnimation` _asboss_mannequin_hand_right_skeleton_anim_blueprint))

(event `self.ReceiveTick`
  (params (DeltaSeconds :type "Float (single-precision)")))

(event `SplayedMovement`
  (bind (_returnvalue_x _returnvalue_y _returnvalue_z) (`KismetMathLibrary.BreakVector` (`BlackboardComponent.GetValueAsVector` (`AIBlueprintHelperLibrary.GetBlackboard` null) "StartingLocation")))
  ;[1 1 1] Movement when doing the splayed hand attack
  (set `self.bSplayedMovementDone` false)
  (bind (_direction _c_splayedhandmotion) (`Timeline|SplayedMovementTimeline` :!via `PlayFromStart`)
    (:`Update`
      (`self.K2_SetActorLocation` (`self.K2_GetPawn`) (`KismetMathLibrary.MakeVector` _returnvalue_x (+ _returnvalue_y _c_splayedhandmotion) _returnvalue_z) false false))
    (:`Finished`
      (set `self.bSplayedMovementDone` true))))

(event `TriggerBossPhase`
  (params (NewState :type "/Game/Blueprints/AI/E_BossAttacks Enum" :default "NewEnumerator0"))
  ;[1 1 1] Playing the proper animation for each phase (this should have gone into its own function really)
  (set `self.CurrentState` NewState)
  (bind (_direction _c_bossattackwindup) (`Timeline|PhaseWindup` :!via `PlayFromStart`)
    (:`Update`
      (switch `/Game/Blueprints/AI/E_BossAttacks` (`self.CurrentState`)
        (:`NewEnumerator0`
          (`self.ReturnToIdleAnimation` _c_bossattackwindup _c_bossattackwindup))
        (:`NewEnumerator1`
          (`self.FistAnimation` _c_bossattackwindup _c_bossattackwindup))
        (:`NewEnumerator2`
          (`self.SplayedAnimation` _c_bossattackwindup _c_bossattackwindup))
        (:`NewEnumerator4`
          (`self.FingerGunAnimation` _c_bossattackwindup _c_bossattackwindup))))))

(fn `Finger Gun Shoot`
  (bind _returnvalue (`self.K2_GetActorLocation` (`self.K2_GetPawn`)))
  (bind (_returnvalue_roll _returnvalue_pitch _returnvalue_yaw) (`KismetMathLibrary.BreakRotator` (`KismetMathLibrary.FindLookAtRotation` _returnvalue (`self.K2_GetActorLocation` (`GameplayStatics.GetPlayerPawn` 0)))))
  (`|SpawnActorFromClass` (`self.Bullet Class`) (`KismetMathLibrary.MakeTransform` (`KismetMathLibrary.MakeVector` (.x (+ _returnvalue (* (`KismetMathLibrary.GetForwardVector` (`KismetMathLibrary.MakeRotator` 0.0 0.0 _returnvalue_yaw)) 1000.0))) (.y (+ _returnvalue (* (`KismetMathLibrary.GetForwardVector` (`KismetMathLibrary.MakeRotator` 0.0 0.0 _returnvalue_yaw)) 1000.0)))) (`KismetMathLibrary.MakeRotator` 0.0 0.0 _returnvalue_yaw)) "Undefined" "OverrideRootScale" null null)
  (`GameplayStatics.PlaySound2D` "/Game/Sounds/sfx_PlayerBullet_Cue.sfx_PlayerBullet_Cue" 1.0 1.0 0.0 null null))

(fn `FingerGunAnimation`
  (params (FingerGunWeight :type "Float (double-precision)") (Alpha :type "Float (double-precision)"))
  (set `/Game/Geometry/Mannequin/Character/Mesh/Boss_MannequinHand_Right_Skeleton_AnimBlueprint.GunWeight` FingerGunWeight (`self.BossAnimation`))
  (`self.K2_SetActorRotation` (`self.K2_GetPawn`) (`KismetMathLibrary.RLerp` (`self.K2_GetActorRotation` (`self.K2_GetPawn`)) (`self.FingerGunRotation`) Alpha) false))

(fn `FistAnimation`
  (params (FistWeight :type "Float (double-precision)") (Alpha :type "Float (double-precision)"))
  (set `/Game/Geometry/Mannequin/Character/Mesh/Boss_MannequinHand_Right_Skeleton_AnimBlueprint.FistWeight` FistWeight (`self.BossAnimation`))
  (`self.K2_SetActorRotation` (`self.K2_GetPawn`) (`KismetMathLibrary.RLerp` (`self.K2_GetActorRotation` (`self.K2_GetPawn`)) (`self.FistRotation`) Alpha) false))

(fn `ReturnToIdleAnimation`
  (params (BlendWeight :type "Float (double-precision)") (Alpha :type "Float (double-precision)"))
  (locals (AdjustedBlendWeight :type "Float (double-precision)"))
  (set `local.AdjustedBlendWeight` (- 1.0 BlendWeight))
  (if (== (`/Game/Geometry/Mannequin/Character/Mesh/Boss_MannequinHand_Right_Skeleton_AnimBlueprint.FistWeight` (`self.BossAnimation`)) 0.0)
    (if (== (`/Game/Geometry/Mannequin/Character/Mesh/Boss_MannequinHand_Right_Skeleton_AnimBlueprint.SplayedWeight` (`self.BossAnimation`)) 0.0)
      (if (not (== (`/Game/Geometry/Mannequin/Character/Mesh/Boss_MannequinHand_Right_Skeleton_AnimBlueprint.GunWeight` (`self.BossAnimation`)) 0.0))
        (set `/Game/Geometry/Mannequin/Character/Mesh/Boss_MannequinHand_Right_Skeleton_AnimBlueprint.GunWeight` (`local.AdjustedBlendWeight`) (`self.BossAnimation`))
        (`self.K2_SetActorRotation` (`self.K2_GetPawn`) (`KismetMathLibrary.RLerp` (`self.K2_GetActorRotation` (`self.K2_GetPawn`)) (`self.InitialRotation`) Alpha) false :!label _label))
      (else
        (set `/Game/Geometry/Mannequin/Character/Mesh/Boss_MannequinHand_Right_Skeleton_AnimBlueprint.SplayedWeight` (`local.AdjustedBlendWeight`) (`self.BossAnimation`))
        (goto _label)))
    (else
      (set `/Game/Geometry/Mannequin/Character/Mesh/Boss_MannequinHand_Right_Skeleton_AnimBlueprint.FistWeight` (`local.AdjustedBlendWeight`) (`self.BossAnimation`))
      (goto _label))))

(fn `ShootFunction`
  (switch `/Game/Blueprints/AI/E_BossAttacks` (`self.CurrentState`)
    (:`NewEnumerator2`
      (`self.Splayed SHot`))
    (:`NewEnumerator4`
      (`self.Finger Gun Shoot`))))

(fn `Splayed SHot`
  (`|SpawnActorFromClass` (`self.Bullet Class`) (`KismetMathLibrary.MakeTransform` (+ (`self.K2_GetActorLocation` (`self.K2_GetPawn`)) (-1000.0 0.0 0.0)) (struct :`Yaw` -180.0 :`Roll` 180.0)) "Undefined" "OverrideRootScale" null null)
  (`|SpawnActorFromClass` (`self.Bullet Class`) (`KismetMathLibrary.MakeTransform` (+ (`self.K2_GetActorLocation` (`self.K2_GetPawn`)) (-500.0 300.0 0.0)) (struct :`Yaw` 160.0)) "Undefined" "OverrideRootScale" null null)
  (`|SpawnActorFromClass` (`self.Bullet Class`) (`KismetMathLibrary.MakeTransform` (+ (`self.K2_GetActorLocation` (`self.K2_GetPawn`)) (-900.0 -300.0 0.0)) (struct :`Yaw` -150.0)) "Undefined" "OverrideRootScale" null null)
  (`GameplayStatics.PlaySound2D` "/Game/Sounds/sfx_PlayerBullet_Cue.sfx_PlayerBullet_Cue" 1.0 1.0 0.0 null null))

(fn `SplayedAnimation`
  (params (SplayedWeight :type "Float (double-precision)") (Alpha :type "Float (double-precision)"))
  (set `/Game/Geometry/Mannequin/Character/Mesh/Boss_MannequinHand_Right_Skeleton_AnimBlueprint.SplayedWeight` SplayedWeight (`self.BossAnimation`))
  (`self.K2_SetActorRotation` (`self.K2_GetPawn`) (`KismetMathLibrary.RLerp` (`self.K2_GetActorRotation` (`self.K2_GetPawn`)) (`self.SplayedRotation`) Alpha) false))

(fn `UserConstructionScript`)